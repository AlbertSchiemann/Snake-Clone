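; BP_SnakeHead is the player-controlled head of a Snake game, moving one mesh-width step on every Tick.
; Input sets the next direction only on the axis perpendicular to the last actual move, which blocks reversing.
; Each tail segment takes the previous location of the piece ahead, following the head as a chain.
; EatFood increments the score shown in WBP_Score and spawns a BP_SnakeTail with the head's mesh.
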(event `InputAction|MoveRight`
  (params (Key :type "Key Structure"))
  (bind (_currentmovedirection_x _currentmovedirection_y) (`KismetMathLibrary.BreakVector` (`self.CurrentMoveDirection`)))
  ;[1 1 1] Change Move Direction
  (:`Pressed`
    (if (== 0.0 _currentmovedirection_y)
      (set `self.MoveDirection` (0.0 1.0 0.0)))))

(event `InputAction|MoveLeft`
  (params (Key :type "Key Structure"))
  (bind (_currentmovedirection_x _currentmovedirection_y) (`KismetMathLibrary.BreakVector` (`self.CurrentMoveDirection`)))
  ;[1 1 1] Change Move Direction
  (:`Pressed`
    (if (== 0.0 _currentmovedirection_y)
      (set `self.MoveDirection` (0.0 -1.0 0.0)))))

(event `InputAction|MoveUp`
  (params (Key :type "Key Structure"))
  (bind _currentmovedirection_x (`KismetMathLibrary.BreakVector` (`self.CurrentMoveDirection`)))
  ;[1 1 1] Change Move Direction
  (:`Pressed`
    (if (== 0.0 _currentmovedirection_x)
      (set `self.MoveDirection` (1.0 0.0 0.0)))))

(event `InputAction|MoveDown`
  (params (Key :type "Key Structure"))
  (bind _currentmovedirection_x (`KismetMathLibrary.BreakVector` (`self.CurrentMoveDirection`)))
  ;[1 1 1] Change Move Direction
  (:`Pressed`
    (if (== 0.0 _currentmovedirection_x)
      (set `self.MoveDirection` (-1.0 0.0 0.0)))))

(event `self.ReceiveBeginPlay`
  (`self.SetLength`)
  (`self.CreateUI`))

(event `self.ReceiveTick`
  (params (DeltaSeconds :type "Float (single-precision)"))
  (`self.Move`))

(event `EatFood`
  (`self.AddScore`)
  (`self.AddTail`))

(fn `AddScore`
  ;[1 1 1] Calculating new Score
  (bind _result (`/Engine/EditorBlueprintResources/StandardMacros.IncrementInt` (`self.Score`))
    (:`  `
      (`/Game/Blueprints/WBP_Score.SetScore` (`self.MainUI`) _result))))

(fn `AddTail`
  (bind _returnvalue (`|SpawnActorFromClass` "/Game/Blueprints/BP_SnakeTail.BP_SnakeTail_C" (`KismetMathLibrary.MakeTransform` (- (`self.K2_GetActorLocation`) (* (`self.MoveDirection`) (`self.StepSize`))) (struct) (0.6 0.6 0.6)) "AlwaysSpawn" "OverrideRootScale" null null))
  (`StaticMeshComponent.SetStaticMesh` (`/Game/Blueprints/BP_ItemParent.Mesh` _returnvalue) (`StaticMeshComponent.StaticMesh` (`self.Head`)))
  (`KismetArrayLibrary.Array_Add` (`self.SnakeTails`) _returnvalue))

(fn `CreateUI`
  (bind _returnvalue (`|CreateWidget` "/Game/Blueprints/WBP_Score.WBP_Score_C" (`GameplayStatics.GetPlayerController` 0)))
  (bind _output_get (set `self.MainUI` _returnvalue))
  (`UserWidget.AddToViewport` _output_get 0))

(fn `Move`
  ;[1 1 1] Move Snake Head
  (set `self.TailPreviousLocation` (`self.K2_GetActorLocation`))
  (`self.K2_AddActorWorldOffset` (* (`self.MoveDirection`) (`self.StepSize`)))
  (set `self.CurrentMoveDirection` (- (`self.K2_GetActorLocation`) (`self.TailPreviousLocation`)))
  ;[1 1 1] Move Tail parts
  (for _array_element (`self.SnakeTails`)
    (bind _output_get (set `self.TailCurrentLocation` (`self.K2_GetActorLocation` _array_element)))
    (`self.K2_SetActorLocation` _array_element (`self.TailPreviousLocation`) false false)
    (set `self.TailPreviousLocation` _output_get)))

(fn `SetLength`
  (bind _returnvalue (`StaticMesh.GetBoundingBox` (`StaticMeshComponent.StaticMesh` (`self.Head`))))
  (set `self.StepSize` (- (.x (`.Max` (break `Box` _returnvalue))) (.x (break `Box` _returnvalue)))))

(fn `UserConstructionScript`)