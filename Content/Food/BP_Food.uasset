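; BP_Food is the food pickup in a Snake clone, consumed when the player overlaps it.
; Its PlayerOvelaped event calls EatFood on the player, has GM_SnakeClone spawn the next food, then destroys the actor.
; After destruction, it also finds the first FT_Eating actor and sets its TestSucess flag, coupling the gameplay Blueprint directly to that test.
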(event `self.PlayerOvelaped`
  (params (Player :type "/Game/Snake/BP_SnakeHead Object Reference"))
  (`/Game/Snake/BP_SnakeHead.EatFood` Player)
  (bind _asgm_snake_clone (cast `/Game/GameMode/GM_SnakeClone` (`GameplayStatics.GetGameMode`)))
  (`/Game/GameMode/GM_SnakeClone.SpawnFood` _asgm_snake_clone)
  (`self.K2_DestroyActor`)
  (bind _outactors (`GameplayStatics.GetAllActorsOfClass` "/Game/UnitTests/FT_Eating.FT_Eating_C"))
  (bind _asft_eating (cast `/Game/UnitTests/FT_Eating` (`|GetArrayItem` _outactors)))
  (set `/Game/UnitTests/FT_Eating.TestSucess` true _asft_eating))

(fn `UserConstructionScript`
  (`parent.UserConstructionScript`))